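; Player-controlled cube that moves under its own simple gravity simulation.
; Each tick it makes a swept move by Velocity, adds Gravity to Velocity, and zeroes Velocity if the move fails.
; Space Bar overrides Velocity with a fixed downward Z value, and the construction script sets Gravity to Earth-like downward acceleration in unscaled Unreal units.
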(event `Key|SpaceBar`
  (:`Pressed`
    (set `self.Velocity` (0.0 0.0 -10.0))))

(event `self.ReceiveTick`
  (params (DeltaSeconds :type "Float (single-precision)"))
  (bind _velocity (`self.Velocity`))
  (bind (_sweephitresult _returnvalue) (`self.K2_SetActorLocation` (+ (* _velocity DeltaSeconds) (`self.K2_GetActorLocation`)) true))
  (set `self.Velocity` (+ (* (`self.Gravity`) DeltaSeconds) _velocity))
  (if (not _returnvalue)
    (set `self.Velocity` (0.0 0.0 0.0))))

(fn `UserConstructionScript`
  (set `self.Gravity` (0.0 0.0 -9.81)))